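; First-person character Blueprint that connects the player to an inventory and a skill system screen.
; On BeginPlay it spawns a player BP_Inventory actor, takes its main widget, fills the skills panel from SkillsSystem and binds key events.
; Key events toggle the inventory and the skills panel, the latter also switching input mode and mouse cursor.
; Taking an item adds it to the inventory, destroying the world actor only when no remainder is left.
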(event Custom|OnTakeToInventoryKeyPressedEvent
  (params (Item :type Interactive%20Items%20Object%20Reference))
  (bind _asbp_takeble_item (Utilities|Casting|CastToBP_TakebleItem Item))
  (bind _rest_ (Default|AddItem (Variables|Default|GetInventoryRef) (.3dblueprint (Variables|/Game/Blueprints/IntaractiveItems/TakebleItems/BP_TakebleItem.BP_TakebleItem_C|GetItemInfo _asbp_takeble_item)) 1))
  (if (== _rest_ 0)
    (Actor|DestroyActor Item)))

(event Custom|OnInventoryKeyPressedEvent
  (bind _inventoryref (Variables|Default|GetInventoryRef))
  (if (Variables|/Game/Blueprints/Inventory/BP_Inventory.BP_Inventory_C|GetisVisible (Variables|Default|GetInventoryRef))
    (Default|HideInventory _inventoryref false)
    (else
      (Default|ShowInventory _inventoryref false))))

(event Custom|OnSkillSystemPressed
  (if (Variables|Default|GetIsSkillSystemVisible)
    (CallFunction|HideSkillSystem)
    (Variables|Default|SetIsSkillSystemVisible false)
    (else
      (CallFunction|ShowSkillSystem)
      (Variables|Default|SetIsSkillSystemVisible true))))

(event EventBeginPlay
  (Variables|Default|SetIsMainWidgetCreated false)
  (bind _returnvalue (Game|SpawnActorfromClass "/Game/Blueprints/Inventory/BP_Inventory.BP_Inventory_C" (Math|Transform|MakeTransform "0, 0, 0" "0, 0, 0" "1,1,1") "AlwaysSpawn" 0 9 self 3 2.0 true (Variables|Default|GetInventory%20Text) true 0))
  (Variables|Default|SetInventoryRef _returnvalue)
  (EventDispatchers|AssignOnTaketoInventoryKeyPressed (delegate Custom|OnTakeToInventoryKeyPressedEvent))
  (EventDispatchers|AssignOnInventoryKeyPressed (delegate Custom|OnInventoryKeyPressedEvent))
  (Variables|Default|SetW_MainWidget (Variables|/Game/Blueprints/Inventory/BP_Inventory.BP_Inventory_C|GetMainWidget (Variables|Default|GetInventoryRef)))
  (Default|HideInventory (Variables|Default|GetInventoryRef) false)
  (Variables|/Game/Blueprints/Widgets/W_SkillsSystem.W_SkillsSystem_C|SetSkills (Variables|/Game/Blueprints/Widgets/W_MainWidget.W_MainWidget_C|GetW_SkillsSystem (Variables|Default|GetW_MainWidget)) (Variables|/Script/SoulExchange.SkillSystem|GetSkills (Variables|Default|GetSkillsSystem)))
  (bind _output_get (Variables|/Game/Blueprints/Widgets/W_MainWidget.W_MainWidget_C|SetW_SkillsSystem (Variables|Default|GetW_MainWidget) (Variables|/Game/Blueprints/Widgets/W_MainWidget.W_MainWidget_C|GetW_SkillsSystem (Variables|Default|GetW_MainWidget))))
  (bind _output_get_2 (Variables|Default|SetW_SkillSystem _output_get))
  (Default|GenerateSlotWidjet _output_get_2)
  (CallFunction|HideSkillSystem)
  (Variables|Default|SetIsSkillSystemVisible false)
  (EventDispatchers|BindEventtoOnSkillSystemKeyPressedEvent (delegate Custom|OnSkillSystemPressed)))

(fn ConstructionScript)

(fn ShowSkillSystem
  (bind _returnvalue (Game|GetPlayerController 0))
  (bind _w_mainwidget (Variables|Default|GetW_MainWidget))
  (bind _w_skillssystem (Variables|/Game/Blueprints/Widgets/W_MainWidget.W_MainWidget_C|GetW_SkillsSystem _w_mainwidget))
  (Widget|SetIsEnabled (Variables|/Game/Blueprints/Widgets/W_MainWidget.W_MainWidget_C|GetW_SkillsSystem (Variables|Default|GetW_MainWidget)) true)
  (Widget|SetVisibility _w_skillssystem "Visible")
  (Input|SetInputModeGameandUI _returnvalue _w_skillssystem "DoNotLock" false)
  (Variables|/Script/Engine.PlayerController|SetbShowMouseCursor _returnvalue true))

(fn HideSkillSystem
  (bind _returnvalue (Game|GetPlayerController 0))
  (Widget|SetIsEnabled (Variables|/Game/Blueprints/Widgets/W_MainWidget.W_MainWidget_C|GetW_SkillsSystem (Variables|Default|GetW_MainWidget)) false)
  (Widget|SetVisibility (Variables|/Game/Blueprints/Widgets/W_MainWidget.W_MainWidget_C|GetW_SkillsSystem (Variables|Default|GetW_MainWidget)) "Hidden")
  (Input|SetInputModeGameOnly _returnvalue)
  (Variables|/Script/Engine.PlayerController|SetbShowMouseCursor _returnvalue false))