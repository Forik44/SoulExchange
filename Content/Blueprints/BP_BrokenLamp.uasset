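; BP_BrokenLamp is a lamp that flickers and goes out the first time something overlaps its Box trigger.
; Audio is stopped at BeginPlay and plays on overlap while IsWork is true.
; A chain of short delays toggles the PointLight off, briefly on, then off for good, after which IsWork is cleared.
; IsWork is only cleared at the end, so overlaps during the sequence can replay the audio.
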(event OnComponentBeginOverlap(Box)
  (params (OverlappedComponent :type Primitive%20Component%20Object%20Reference) (OtherActor :type Actor%20Object%20Reference) (OtherComp :type Primitive%20Component%20Object%20Reference) (OtherBodyIndex :type Integer) (bFromSweep :type Boolean) (SweepResult :type Hit%20Result%20Structure%20%28by%20ref%29))
  (if (Variables|Default|GetIsWork)
    (Audio|Components|Audio|Play (Variables|Default|GetAudio) 0.0)
    (Utilities|FlowControl|Delay 1.1)
    (Rendering|SetVisibility (Variables|Default|GetPointLight) false false)
    (Utilities|FlowControl|Delay 0.1)
    (Rendering|SetVisibility (Variables|Default|GetPointLight) true false)
    (Utilities|FlowControl|Delay 0.05)
    (Rendering|SetVisibility (Variables|Default|GetPointLight) false false)
    (Variables|Default|SetIsWork false)))

(event EventBeginPlay
  (Audio|Components|Audio|Stop (Variables|Default|GetAudio)))

(event Collision|EventActorBeginOverlap
  (params (OtherActor :type Actor%20Object%20Reference)))

(event EventTick
  (params (DeltaSeconds :type Float%20%28single-precision%29)))

(fn ConstructionScript)