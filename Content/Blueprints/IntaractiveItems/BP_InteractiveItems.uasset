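; BP_InteractiveItems is an interactive item that displays a text message when used.
; On BeginPlay it binds a handler to the OnUseKeyPressed dispatcher.
; The handler writes TextToShow into the W_TextWidget held by its WidgetText component, shows it, then hides it after a short delay.
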(event Custom|OnUseKeyPressedEvent
  (bind _widgettext (Variables|Default|GetWidgetText))
  (bind _output_get (Variables|Default|SetWidget_Prom (UserInterface|GetUserWidgetObject (Variables|Default|GetWidgetText))))
  (bind _asbp_text_widget (Utilities|Casting|CastToW_TextWidget _output_get))
  (Variables|/Game/Blueprints/Widgets/W_TextWidget.W_TextWidget_C|SetContent _asbp_text_widget (Variables|Default|GetText%20To%20Show))
  (Rendering|SetVisibility _widgettext true false)
  (Utilities|FlowControl|Delay 4.0)
  (Rendering|SetVisibility _widgettext false false))

(event EventBeginPlay
  (EventDispatchers|AssignOnUseKeyPressed (delegate Custom|OnUseKeyPressedEvent)))

(fn ConstructionScript)