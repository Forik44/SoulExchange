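; BP_Door is an interactive door Blueprint that swings open and shut and can be locked with a key.
; OpenDoorWithKey clears IsClosed and calls OpenDoor when both the key and its ID match; OpenDoor only works on an unlocked door.
; RotateDoor plays or reverses the DoorRotation timeline based on its current value, applying that value as relative yaw to both Door and Handle.
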(event Custom|RotateDoor
  (if (< (stale _doorrotaton) 1.0)
    (bind _doorrotaton (Timeline|DoorRotation Play)
      (:Update
        (Transformation|SetRelativeRotation (Variables|Default|GetDoor) (Math|Rotator|MakeRotator 0.0 0.0 _doorrotaton) false false)
        (Transformation|SetRelativeRotation (Variables|Default|GetHandle) (Math|Rotator|MakeRotator 0.0 0.0 _doorrotaton) false false)))
    (else
      (Timeline|DoorRotation Reverse))))

(event EventBeginPlay
  (|CallParentFunction) ; This node is disabled and will not be called.\nDrag off pins to build functionality.
)

(event Collision|EventActorBeginOverlap
  (params (OtherActor :type Actor%20Object%20Reference)))

(event EventTick
  (params (DeltaSeconds :type Float%20%28single-precision%29)))

(fn ConstructionScript
  (|CallParentFunction))

(fn OpenDoorwithKey
  (params (Key :type BP%20Interactive%20Items%20Class%20Reference) (KeyID :type Integer))
  (if (Variables|Default|GetIsClosed)
    (if (and (== Key (Variables|Default|GetBP_Key)) (== KeyID (Variables|Default|GetIDKey)))
      (Variables|Default|SetIsClosed false)
      (CallFunction|OpenDoor))))

(fn OpenDoor
  (if (not (Variables|Default|GetIsClosed))
    (CallFunction|RotateDoor)))