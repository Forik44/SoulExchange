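; BP_OpenerDistDoor is a keycard-gated opener that drives a referenced DistDoor.
; OpenDoorWithCard opens the door when the card level meets or exceeds LevelCard, and ignores requests while IsDelay is set.
; An exact level match with IsTimer instead runs OpenDoorWithTimer, which calls OpenDoor(true) before and after a delay, holding IsDelay throughout.
; Higher-level cards always skip the timer.
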(event Custom|OpenDoorWithTimer
  (Default|OpenDoor (Variables|Default|GetDistDoor) true)
  (Variables|Default|SetIsDelay true)
  (Utilities|FlowControl|Delay (Variables|Default|GetDelay))
  (Default|OpenDoor (Variables|Default|GetDistDoor) true)
  (Variables|Default|SetIsDelay false))

(event EventBeginPlay
  (|CallParentFunction) ; This node is disabled and will not be called.\nDrag off pins to build functionality.
)

(event Collision|EventActorBeginOverlap
  (params (OtherActor :type Actor%20Object%20Reference)))

(event EventTick
  (params (DeltaSeconds :type Float%20%28single-precision%29)))

(fn ConstructionScript
  (|CallParentFunction))

(fn OpenDoorwithCard
  (params (CardLevel :type Integer))
  (bind _levelcard (Variables|Default|GetLevelCard))
  (bind _returnvalue (== CardLevel _levelcard))
  (if (not (Variables|Default|GetIsDelay))
    (if (and _returnvalue (Variables|Default|GetIsTimer))
      (CallFunction|OpenDoorwithTimer)
      (elif _returnvalue
        (Default|OpenDoor (Variables|Default|GetDistDoor) true :!label _label)
        (elif (> CardLevel (Variables|Default|GetLevelCard))
          (goto _label))))))