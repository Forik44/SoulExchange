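; BP_BedSide_Table is an interactive bedside table whose top and bottom shelves slide open and shut together.
; OpenCabinet calls OpenCabinetEvent, which plays or reverses a timeline based on its current Location value rather than on IsOpen.
; The timeline drives the relative X location of both shelf components.
; IsOpen is set by the event, then immediately flipped again by OpenCabinet.
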(event Custom|OpenCabinetEvent
  (if (> (stale _location) -0.3)
    (Variables|Default|SetIsOpen false)
    (bind _location (Timeline|Timeline_0 Play)
      (:Update
        (Transformation|SetRelativeLocation (Variables|Default|GetBedside_Table_Shelf_Top) (Math|Vector|MakeVector _location 0.0 0.0) false false)
        (Transformation|SetRelativeLocation (Variables|Default|GetBedside_Table_Shelf_Bottom) (Math|Vector|MakeVector _location 0.0 0.0) false false)))
    (else
      (Variables|Default|SetIsOpen true)
      (Timeline|Timeline_0 Reverse))))

(event EventBeginPlay
  (|CallParentFunction) ; This node is disabled and will not be called.\nDrag off pins to build functionality.
)

(event Collision|EventActorBeginOverlap
  (params (OtherActor :type Actor%20Object%20Reference))
  (|CallParentFunction OtherActor) ; This node is disabled and will not be called.\nDrag off pins to build functionality.
)

(event EventTick
  (params (DeltaSeconds :type Float%20%28single-precision%29))
  (|CallParentFunction DeltaSeconds) ; This node is disabled and will not be called.\nDrag off pins to build functionality.
)

(fn ConstructionScript
  (|CallParentFunction))

(fn OpenCabinet
  (CallFunction|OpenCabinetEvent)
  (if (Variables|Default|GetIsOpen)
    (Variables|Default|SetIsOpen false)
    (else
      (Variables|Default|SetIsOpen true))))