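; BP_DefaultCloset is an interactive storage cabinet whose drawer slides open and closed with sound.
; On BeginPlay it calls GenerateInventory with the player's BP_FPCharacter and silences both sounds.
; OpenCabinet triggers a timeline that plays or reverses based on its current value, moving the shelf and knob along relative Y.
; The resulting IsOpen flag selects the open or close sound.
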(event Custom|OpenCabinetEvent
  (if (< (stale _location) 1.0)
    (Variables|Default|SetIsOpen true)
    (bind _location (Timeline|LocationDoors Play)
      (:Update
        (Transformation|SetRelativeLocation (Variables|Default|GetCabinet_lp_Shelf_lp) (Math|Vector|MakeVector 0.0 _location 0.0) false false)
        (Transformation|SetRelativeLocation (Variables|Default|GetCabinet_lp_Knob_lp) (Math|Vector|MakeVector 0.0 _location 0.0) false false)))
    (else
      (Variables|Default|SetIsOpen false)
      (Timeline|LocationDoors Reverse))))

(event EventBeginPlay
  (bind _returnvalue (Game|GetPlayerCharacter 0))
  (bind (_asbp_fpcharacter _bsuccess) (Utilities|Casting|CastToBP_FPCharacter _returnvalue))
  (|CallParentFunction)
  (if _bsuccess
    (CallFunction|GenerateInventory _asbp_fpcharacter)
    (Audio|Components|Audio|Stop (Variables|Default|GetOpenSound))
    (Audio|Components|Audio|Stop (Variables|Default|GetCloseSound))))

(event Collision|EventActorBeginOverlap
  (params (OtherActor :type Actor%20Object%20Reference)))

(event EventTick
  (params (DeltaSeconds :type Float%20%28single-precision%29)))

(fn ConstructionScript
  (|CallParentFunction))

(fn OpenCabinet
  (CallFunction|OpenCabinetEvent)
  (if (Variables|Default|GetIsOpen)
    (Audio|Components|Audio|Play (Variables|Default|GetOpenSound) 0.0)
    (else
      (Audio|Components|Audio|Play (Variables|Default|GetCloseSound) 0.0))))