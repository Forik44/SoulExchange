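; Bathroom locker container that the player can open and close, found among the game's interactive chest items.
; On BeginPlay it generates its inventory from the player's BP_FPCharacter, then stops its Open and Close components so neither plays at start.
; OpenCabinet toggles IsOpen and plays Open or Close from the start to match the new state.
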(event EventBeginPlay
  (bind _returnvalue (Game|GetPlayerCharacter 0))
  (bind (_asbp_fpcharacter _bsuccess) (Utilities|Casting|CastToBP_FPCharacter _returnvalue))
  (|CallParentFunction)
  (if _bsuccess
    (CallFunction|GenerateInventory _asbp_fpcharacter)
    (Audio|Components|Audio|Stop (Variables|Default|GetOpen))
    (Audio|Components|Audio|Stop (Variables|Default|GetClose))))

(event Collision|EventActorBeginOverlap
  (params (OtherActor :type Actor%20Object%20Reference))
  (|CallParentFunction OtherActor) ; This node is disabled and will not be called.\nDrag off pins to build functionality.
)

(event EventTick
  (params (DeltaSeconds :type Float%20%28single-precision%29))
  (|CallParentFunction DeltaSeconds) ; This node is disabled and will not be called.\nDrag off pins to build functionality.
)

(fn ConstructionScript
  (|CallParentFunction))

(fn OpenCabinet
  (if (Variables|Default|GetIsOpen)
    (Variables|Default|SetIsOpen false)
    (else
      (Variables|Default|SetIsOpen true)))
  (if (Variables|Default|GetIsOpen)
    (Audio|Components|Audio|Play (Variables|Default|GetOpen) 0.0)
    (else
      (Audio|Components|Audio|Play (Variables|Default|GetClose) 0.0))))