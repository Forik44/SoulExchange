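; BP_DefaultKey is a takeable key item that, when used, tries to open the door the player is looking at.
; On use, it runs a short Visibility line trace forward from the player character's camera, ignoring the player.
; A hit BP_Door receives the key's class and ID through OpenDoorWithKey; otherwise the inventory action menu's IsWorked flag is set to false.
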(event EventBeginPlay
  (|CallParentFunction) ; This node is disabled and will not be called.\nDrag off pins to build functionality.
)

(event Collision|EventActorBeginOverlap
  (params (OtherActor :type Actor%20Object%20Reference))
  (|CallParentFunction OtherActor) ; This node is disabled and will not be called.\nDrag off pins to build functionality.
)

(event EventTick
  (params (DeltaSeconds :type Float%20%28single-precision%29))
  (|CallParentFunction DeltaSeconds) ; This node is disabled and will not be called.\nDrag off pins to build functionality.
)

(event EventEventonUsed
  (bind _returnvalue (Game|GetPlayerCharacter 0))
  (bind _asbp_fpcharacter (Utilities|Casting|CastToBP_FPCharacter _returnvalue))
  (bind _returnvalue_2 (Actor|GetComponentsByClass _asbp_fpcharacter "/Script/Engine.CameraComponent"))
  (bind _output (Utilities|Array|Get(acopy) _returnvalue_2))
  (bind _returnvalue_3 (Transformation|GetWorldLocation _output))
  (bind _outhit (Collision|LineTraceByChannel _returnvalue_3 (+ _returnvalue_3 (* (Math|Vector|GetForwardVector _output) 4e+02)) "TraceTypeQuery1" false (Utilities|Array|MakeArray _asbp_fpcharacter) "None"))
  (bind _asbp_door (Utilities|Casting|CastToBP_Door (.hitactor _outhit))
    (:then
      (Default|OpenDoorwithKey _asbp_door (Utilities|GetClass self) (Variables|Default|GetIDKey)))
    (:CastFailed
      (Variables|/Game/Blueprints/Inventory/W_ActionMenu.W_ActionMenu_C|SetIsWorked (Variables|/Game/Blueprints/Inventory/W_Inventory.W_Inventory_C|GetW_ActionMenu (Variables|/Game/Blueprints/Widgets/W_MainWidget.W_MainWidget_C|GetW_InventoryWidget (Variables|/Game/Blueprints/BP_FPCharacter.BP_FPCharacter_C|GetW_MainWidget (.AsBP%20FPCharacter (Utilities|Casting|CastToBP_FPCharacter (Game|GetPlayerCharacter 0)))))) false))))

(fn ConstructionScript
  (|CallParentFunction))