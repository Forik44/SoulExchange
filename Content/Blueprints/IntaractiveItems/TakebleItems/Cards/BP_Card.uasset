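; BP_Card is a key card item that opens card-locked doors.
; When used, it runs a short Visibility line trace forward from the player character's camera, ignoring the player.
; If the trace hits a BP_OpenerDistDoor, it passes its CardLevel to that actor's OpenDoorWithCard, leaving the response to the opener.
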(event EventBeginPlay
  (|CallParentFunction) ; This node is disabled and will not be called.\nDrag off pins to build functionality.
)

(event EventEventonUsed
  (bind _returnvalue (Game|GetPlayerCharacter 0))
  (bind _asbp_fpcharacter (Utilities|Casting|CastToBP_FPCharacter _returnvalue))
  (bind _returnvalue_2 (Actor|GetComponentsByClass _asbp_fpcharacter "/Script/Engine.CameraComponent"))
  (bind _output (Utilities|Array|Get(acopy) _returnvalue_2))
  (bind _returnvalue_3 (Transformation|GetWorldLocation _output))
  (bind _outhit (Collision|LineTraceByChannel _returnvalue_3 (+ _returnvalue_3 (* (Math|Vector|GetForwardVector _output) 1e+02)) "TraceTypeQuery1" false (Utilities|Array|MakeArray _asbp_fpcharacter) "None"))
  (bind _asbp_opener_dist_door (Utilities|Casting|CastToBP_OpenerDistDoor (.hitactor _outhit)))
  (Default|OpenDoorwithCard _asbp_opener_dist_door (Variables|Default|GetCardLevel)))

(fn ConstructionScript
  (|CallParentFunction))