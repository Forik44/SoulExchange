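; Game instance Blueprint that applies saved sound volume settings through the SetGameSound event.
; It sets SCM_Main as the base sound mix, then loads the SaveSoundSettings slot if it exists and applies main, menu music and effects volumes as sound class overrides.
; A failed cast attempts full-volume defaults through the invalid cast result, while a missing save leaves the class volumes untouched.
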(event Custom|SetGameSound
  (Class|GameplayStatics|SetBaseSoundMix "/Game/Sounds/Music/SCM_Main.SCM_Main")
  (bind _returnvalue (SaveGame|DoesSaveGameExist "SaveSoundSettings"))
  (if _returnvalue
    (bind _returnvalue_2 (SaveGame|LoadGamefromSlot "SaveSoundSettings"))
    (bind _output_get (Variables|Default|SetSaveSoundSettingsRef _returnvalue_2))
    (bind _asbp_save_settings_sounds (Utilities|Casting|CastToBP_SaveSettingsSounds _output_get)
      (:then
        (Audio|SetSoundMixClassOverride "/Game/Sounds/Music/SCM_Main.SCM_Main" "/Game/Sounds/Music/SC_MainMusic.SC_MainMusic" (Variables|/Game/Blueprints/BP_SaveSettingsSounds.BP_SaveSettingsSounds_C|GetMainMenuMusicVolume _asbp_save_settings_sounds) 1.0 1.0 true)
        (Audio|SetSoundMixClassOverride "/Game/Sounds/Music/SCM_Main.SCM_Main" "/Game/Sounds/Music/SC_Main.SC_Main" (Variables|/Game/Blueprints/BP_SaveSettingsSounds.BP_SaveSettingsSounds_C|GetMainVolume _asbp_save_settings_sounds) 1.0 1.0 true)
        (Audio|SetSoundMixClassOverride "/Game/Sounds/Music/SCM_Main.SCM_Main" "/Game/Sounds/Music/SC_Effects.SC_Effects" (Variables|/Game/Blueprints/BP_SaveSettingsSounds.BP_SaveSettingsSounds_C|GetEffectsVolume _asbp_save_settings_sounds) 1.0 1.0 true))
      (:CastFailed
        (bind _output_get_2 (Variables|/Game/Blueprints/BP_SaveSettingsSounds.BP_SaveSettingsSounds_C|SetEffectsVolume _asbp_save_settings_sounds 1.0))
        (Audio|SetSoundMixClassOverride "/Game/Sounds/Music/SCM_Main.SCM_Main" "/Game/Sounds/Music/SC_Effects.SC_Effects" _output_get_2 1.0 1.0 true)
        (bind _output_get_3 (Variables|/Game/Blueprints/BP_SaveSettingsSounds.BP_SaveSettingsSounds_C|SetMainMenuMusicVolume _asbp_save_settings_sounds 1.0))
        (Audio|SetSoundMixClassOverride "/Game/Sounds/Music/SCM_Main.SCM_Main" "/Game/Sounds/Music/SC_MainMusic.SC_MainMusic" _output_get_3 1.0 1.0 true)
        (bind _output_get_4 (Variables|/Game/Blueprints/BP_SaveSettingsSounds.BP_SaveSettingsSounds_C|SetMainVolume _asbp_save_settings_sounds 1.0))
        (Audio|SetSoundMixClassOverride "/Game/Sounds/Music/SCM_Main.SCM_Main" "/Game/Sounds/Music/SC_Main.SC_Main" _output_get_4 1.0 1.0 true)))))